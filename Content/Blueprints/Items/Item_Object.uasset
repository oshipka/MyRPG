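; Item_Object is an inventory item data object exposing an item's grid dimensions, icon, class and ground-clamp flag through getter functions.
; The icon getter returns a rotated icon variant when the item is flagged as rotated.
; The item class and clamp flag are stored alongside it, with the clamp flag indicating whether the item must snap to the ground.
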(fn `Get clamp`
  (returns (`Has to clamp to ground` :type Boolean))
  (return (`self.Has to clamp to ground`)))

(fn `Get Dimensions`
  (returns (Dimensions :type "IntPoint Structure"))
  (return (`self.Dimensions`)))

(fn `Get Icon`
  (returns (Icon :type "MaterialInterface Object Reference"))
  (return (select `bool` (`self.IsRotated`) :`false` (`self.Icon`) :`true` (`self.Icon_Rotated`))))

(fn `Get item class`
  (returns (`Item class` :type "/Game/Blueprints/Items/Item_Class Class Reference"))
  (return (`self.ItemClass`)))