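; Base pickup item actor that shows a widget on overlap and can be added to the player's inventory.
; On BeginPlay it fills a missing ItemObject from GetDefaultItemObject, an empty stub here, and binds to the widget's progress-full event.
; Interact begin and end drive the widget's hold progress.
; PickUpItem passes ItemObject to the player's InventoryComponent and destroys the actor if adding succeeds.
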(event `self.ReceiveBeginPlay`
  (if (not (`KismetSystemLibrary.IsValid` (`self.ItemObject`)))
    (bind _item_object (`self.Get Default Item Object`))
    (set `self.ItemObject` _item_object))
  (bind _aspick_up_widget (cast `/Game/Blueprints/UI/ActivePlaystateHUD/InteractionInterface/PickUpWidget` (`WidgetComponent.GetUserWidgetObject` (`self.Widget`))))
  (add `/Game/Blueprints/UI/ActivePlaystateHUD/InteractionInterface/PickUpWidget.OnProgressBarFull` _aspick_up_widget (`|CreateDelegate` :!event `PickUpItem`)))

(event `/Game/Blueprints/UI/ActivePlaystateHUD/InteractionInterface/InteractInterface.OnOverlapBegin`
  (`SceneComponent.SetVisibility` (`self.Widget`) true true))

(event `/Game/Blueprints/UI/ActivePlaystateHUD/InteractionInterface/InteractInterface.OnOverlapEnd`
  (`SceneComponent.SetVisibility` (`self.Widget`) false true))

(event `/Game/Blueprints/UI/ActivePlaystateHUD/InteractionInterface/InteractInterface.OnInteractBegin`
  (bind _aspick_up_widget (cast `/Game/Blueprints/UI/ActivePlaystateHUD/InteractionInterface/PickUpWidget` (`WidgetComponent.GetUserWidgetObject` (`self.Widget`))))
  (`/Game/Blueprints/UI/ActivePlaystateHUD/InteractionInterface/PickUpWidget.BeginProgress` _aspick_up_widget))

(event `/Game/Blueprints/UI/ActivePlaystateHUD/InteractionInterface/InteractInterface.OnInteractEnd`
  (bind _aspick_up_widget (cast `/Game/Blueprints/UI/ActivePlaystateHUD/InteractionInterface/PickUpWidget` (`WidgetComponent.GetUserWidgetObject` (`self.Widget`))))
  (`/Game/Blueprints/UI/ActivePlaystateHUD/InteractionInterface/PickUpWidget.EndProgress` _aspick_up_widget))

(fn `Get Default Item Object`
  (returns (`Item Object` :type "/Game/Blueprints/Items/Item_Object Object Reference"))
  (return null))

(fn `PickUpItem`
  (bind _added (`/Game/Blueprints/ThirdPersonBp/InventoryComponent.Try Add Item` (`/Game/Blueprints/ThirdPersonBp/MyPlayerCharacter.InventoryComponent` (cast `/Game/Blueprints/ThirdPersonBp/MyPlayerCharacter` (`GameplayStatics.GetPlayerCharacter` 0) :!pure true)) (`self.ItemObject`)))
  (if _added
    (`self.K2_DestroyActor`)))

(fn `UserConstructionScript`)