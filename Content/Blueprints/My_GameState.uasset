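; My_GameState is a game state Blueprint that provides a function for spawning an item into the world in front of a given actor.
; SpawnItemFromActor offsets the spawn point along the actor's forward vector, optionally snapping it to the surface below with a downward Visibility line trace.
; It then spawns the class returned by the item object's GetItemClass, passing that object into the new actor.
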(fn `Spawn item from actor`
  (params (Actor :type "Actor Object Reference") (`Item Object` :type "/Game/Blueprints/Items/Item_Object Object Reference") (`Ground clamp` :type Boolean))
  (locals (`Spawn location (local)` :type "Vector Structure" :default (0.0 0.0 0.0)))
  (bind _actor (`local.Actor`))
  (bind _item_object (`local.Item Object`))
  (`|ExecutionSequence`
    (:`then_0`
      (set `local.Spawn location (local)` (+ (`self.K2_GetActorLocation` _actor) (* (`self.GetActorForwardVector` _actor) 150.0)))
      (if (`local.Ground clamp`)
        (bind (_outhit _returnvalue) (`KismetSystemLibrary.LineTraceSingle` (`local.Spawn location (local)`) (- (`local.Spawn location (local)`) (0.0 0.0 10000000.0)) "TraceTypeQuery1"))
        (if _returnvalue
          (set `local.Spawn location (local)` (`.Location` (`GameplayStatics.BreakHitResult` _outhit))))))
    (:`then_1`
      (`|SpawnActorFromClass` (`/Game/Blueprints/Items/Item_Object.Get item class` _item_object) (`KismetMathLibrary.MakeTransform` (`local.Spawn location (local)`)) "Undefined" "OverrideRootScale" null _item_object null))))

(fn `UserConstructionScript`)