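; Actor component that opens and closes the inventory window through a single toggle function.
; Opening creates an InventoryBP widget bound to this component and adds it to the player controller's HUD canvas, auto-sized, center-aligned and anchored by the Position variable.
; Input switches to UI-only with the mouse locked while the window is open.
; Closing removes the widget, clears the reference and restores game-only input.
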(fn `Toggle inventory`
  (bind _returnvalue (`GameplayStatics.GetPlayerController` 0))
  (`self.Inventory window`
    (:`then`
      (`Widget.RemoveFromParent` (`self.Inventory window`))
      (set `self.Inventory window` null)
      (`WidgetBlueprintLibrary.SetInputMode_GameOnly` _returnvalue))
    (:`else`
      (bind _returnvalue_2 (`|CreateWidget` "/Game/Blueprints/InventorySystem/InventoryInterface/InventoryBP.InventoryBP_C" null self))
      (bind _output_get (set `self.Inventory window` _returnvalue_2))
      (bind _asmy_player_controller (cast `/Game/Blueprints/MyPlayerController` _returnvalue))
      (bind _returnvalue_3 (`CanvasPanel.AddChildToCanvas` (`/Game/Blueprints/HUD.HUDCanvasPanel` (`/Game/Blueprints/MyPlayerController.HudWidget` _asmy_player_controller)) _output_get))
      (`CanvasPanelSlot.SetAutoSize` _returnvalue_3 true)
      (`CanvasPanelSlot.SetAlignment` _returnvalue_3 (0.5 0.5))
      (`CanvasPanelSlot.SetAnchors` _returnvalue_3 (`self.Position`))
      (`WidgetBlueprintLibrary.SetInputMode_UIOnlyEx` (`GameplayStatics.GetPlayerController` 0) (`self.Inventory window`) "LockAlways"))))