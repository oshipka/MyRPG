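; NPC spawner actor that populates its Bound volume with SpawnAmount pawns of a chosen Class.
; Each spawn traces down from above a random point in the bounds to WorldStatic geometry, with debug drawing, and places the pawn just above the hit.
; Pawns receive a default controller and a SpawnPoint back-reference, and join ActivePawns.
; A looping timer refills ActivePawns to SpawnAmount; nothing here removes entries.
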(event `self.ReceiveBeginPlay`
  (for _ (range 1 (+ (`self.Spawn amount`) 1))
    (`self.spawn character`))
  (`KismetSystemLibrary.K2_SetTimer` null "Respawn character" (`self.Time to respawn`) true))

(fn `Respawn character`
  (locals (`mobs to respawn` :type Integer :default 0))
  (bind _output_get (set `local.mobs to respawn` (- (`self.Spawn amount`) (`KismetArrayLibrary.Array_Length` (`self.Active pawns`)))))
  (if (> _output_get 0)
    (for _ (range 1 (+ (`local.mobs to respawn`) 1))
      (`self.spawn character`))))

(fn `spawn character`
  (bind (_origin _boxextent) (`KismetSystemLibrary.GetComponentBounds` (`self.Bound`)))
  (bind _returnvalue (`KismetMathLibrary.MakeVector` (.x (`KismetMathLibrary.RandomPointInBoundingBox` _origin _boxextent)) (.y (`KismetMathLibrary.RandomPointInBoundingBox` _origin _boxextent)) (+ (.z (`KismetMathLibrary.RandomPointInBoundingBox` _origin _boxextent)) 500.0)))
  (bind _outhit (`KismetSystemLibrary.LineTraceSingleForObjects` :`Start` _returnvalue :`End` (+ _returnvalue (* (* (`self.GetActorUpVector`) -1) 15000.0)) :`ObjectTypes` (`|MakeArray` "ObjectTypeQuery1" :!type "EObjectTypeQuery Enum") :`DrawDebugType` "ForDuration"))
  (bind _returnvalue_2 (`|SpawnActorFromClass` (`self.Class`) (`KismetMathLibrary.MakeTransform` (`KismetMathLibrary.MakeVector` (.x (`.Location` (`GameplayStatics.BreakHitResult` _outhit))) (.y (`.Location` (`GameplayStatics.BreakHitResult` _outhit))) (+ (.z (`.Location` (`GameplayStatics.BreakHitResult` _outhit))) 100.0)) (`KismetMathLibrary.MakeRotator` 0.0 0.0 (`KismetMathLibrary.RandomFloat`))) "AdjustIfPossibleButAlwaysSpawn" "OverrideRootScale" null null))
  (`Pawn.SpawnDefaultController` _returnvalue_2)
  (`KismetArrayLibrary.Array_Add` (`self.Active pawns`) _returnvalue_2)
  (set `/Game/Blueprints/NPC/Actors/NpcBase.Spawn point ` self _returnvalue_2))

(fn `UserConstructionScript`)