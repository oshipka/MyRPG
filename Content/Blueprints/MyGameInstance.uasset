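; Game instance that sets up the player's equipment and inventory and the auto-save data on Init.
; It casts player 0's character to MyPlayerCharacter and calls InitEquipmentAndInventory on it; a failed cast also skips the save setup.
; It then loads the SaveSlotAuto slot into SaveGameData, or creates a new MySaveGameObject when no save exists, without writing it to disk.
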(event `self.ReceiveInit`
  (bind _asmy_player_character (cast `/Game/Blueprints/ThirdPersonBp/MyPlayerCharacter` (`GameplayStatics.GetPlayerCharacter` 0)))
  (`/Game/Blueprints/ThirdPersonBp/MyPlayerCharacter.Init Equipment and Inventory` _asmy_player_character)
  (bind _returnvalue (`GameplayStatics.DoesSaveGameExist` (`self.SaveSlot_Auto`)))
  (if _returnvalue
    (bind _returnvalue_2 (`GameplayStatics.LoadGameFromSlot` (`self.SaveSlot_Auto`)))
    (bind _asmy_save_game_object (cast `/Game/Blueprints/MySaveGameObject` _returnvalue_2))
    (set `self.SaveGameData` _asmy_save_game_object)
    (else
      (bind _returnvalue_3 (`GameplayStatics.CreateSaveGameObject` "/Game/Blueprints/MySaveGameObject.MySaveGameObject_C"))
      (set `self.SaveGameData` _returnvalue_3))))